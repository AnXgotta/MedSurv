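; BP_SurvCharacter is a survival character Blueprint with hooks for player status and inventory changes.
; Its events and construction script are empty stubs, leaving PlayerStatusLookAtCamera as the only logic.
; That function places an actor, by name likely the status display, ahead of and slightly below FollowCamera.
; It derives rotation from a look-at toward the camera, inverting pitch and turning yaw half a circle.
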(event Custom|SpawnPlayerStatus_Event)

(event EventBeginPlay)

(event EventEventInventoryDataChanged)

(event EventEventPlayerStatusChanged)

(event EventEventInventoryOpenedClosed
  (params (Open :type Boolean)))

(fn ConstructionScript)

(fn PlayerStatusLookatCamera
  (bind _returnvalue (Transformation|GetActorLocation))
  (bind _followcamera (Variables|Default|GetFollowCamera))
  (bind _returnvalue_2 (Transformation|GetWorldLocation _followcamera))
  (bind _returnvalue_3 (Math|Rotator|FindLookatRotation _returnvalue _returnvalue_2))
  (Transformation|SetActorLocation (- (+ _returnvalue_2 (* (Math|Vector|GetForwardVector _followcamera) 1e+02)) (* (Math|Vector|GetUpVector _followcamera) 25.0)) false false)
  (Transformation|SetActorRotation (Math|Rotator|MakeRotator (.roll _returnvalue_3) (* (.pitch _returnvalue_3) -1.0) (+ (.yaw _returnvalue_3) 1.8e+02))))